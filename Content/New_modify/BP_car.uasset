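; BP_car is a drivable wheeled vehicle pawn with throttle, steering and switchable back and first-person cameras.
; Each tick it feeds a scaled steer angle from the more-turned of wheels 0 and 1 into ABP_car's Steer.
; Switching deactivates one camera, whose deactivation event activates the other.
; A trigger box shows a hint and flags overlap for MotionControllerPawn, while both Handbrake press and release set the handbrake false.
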(event `self.ReceiveTick`
  (params (DeltaSeconds :type "Float (single-precision)"))
  (bind _wheels (`WheeledVehicleMovementComponent.Wheels` (`self.VehicleMovement`)))
  (bind _returnvalue (`VehicleWheel.GetSteerAngle` (`|GetArrayItem` _wheels 1)))
  (bind _returnvalue_2 (`VehicleWheel.GetSteerAngle` (`|GetArrayItem` _wheels)))
  (set `/Game/New_modify/ABP_car.steer` (* 6.428571 (`KismetMathLibrary.SelectFloat` _returnvalue_2 _returnvalue (> (`KismetMathLibrary.Abs` _returnvalue_2) (`KismetMathLibrary.Abs` _returnvalue)))) (`self.As ABP Car`)))

(event `self.BackCamera.OnComponentDeactivated`
  (params (Component :type "ActorComponent Object Reference"))
  (`ActorComponent.Activate` (`self.FirstPersonCamera`) false))

(event `self.FirstPersonCamera.OnComponentDeactivated`
  (params (Component :type "ActorComponent Object Reference"))
  (`ActorComponent.Activate` (`self.BackCamera`) false))

(event `self.ReceiveBeginPlay`
  (bind _asabp_car (cast `/Game/New_modify/ABP_car` (`SkeletalMeshComponent.GetAnimInstance` (`self.Mesh`))))
  (set `self.As ABP Car` _asabp_car))

(event `CustomEvent`)

(event `InputAxis|MoveForward`
  (params (AxisValue :type "Float (single-precision)"))
  (`WheeledVehicleMovementComponent.SetThrottleInput` (`self.VehicleMovement`) AxisValue))

(event `InputAction|SwitchCamera`
  (params (Key :type "Key Structure"))
  (bind _backcamera (`self.BackCamera`))
  (:`Pressed`
    (if (`ActorComponent.IsActive` _backcamera)
      (`ActorComponent.Deactivate` _backcamera)
      (else
        (`ActorComponent.Deactivate` (`self.FirstPersonCamera`))))))

(event `InputAction|Handbrake`
  (params (Key :type "Key Structure"))
  (bind _vehiclemovement (`self.VehicleMovement`))
  (:`Pressed`
    (`WheeledVehicleMovementComponent.SetHandbrakeInput` _vehiclemovement false))
  (:`Released`
    (`WheeledVehicleMovementComponent.SetHandbrakeInput` _vehiclemovement false)))

(event `InputAxis|MoveRight`
  (params (AxisValue :type "Float (single-precision)"))
  (`WheeledVehicleMovementComponent.SetSteeringInput` (`self.VehicleMovement`) AxisValue))

(event `self.EntetCarTriggerBox.OnComponentBeginOverlap`
  (params (OverlappedComponent :type "PrimitiveComponent Object Reference") (OtherActor :type "Actor Object Reference") (OtherComp :type "PrimitiveComponent Object Reference") (OtherBodyIndex :type Integer) (bFromSweep :type Boolean) (SweepResult :type "HitResult Structure (by ref)"))
  (cast `/Game/VR_BP/MotionControllerPawn` OtherActor)
  (`SceneComponent.SetVisibility` (`self.Hint`) true false)
  (set `self.IsOverLapped?` true))

(event `self.EntetCarTriggerBox.OnComponentEndOverlap`
  (params (OverlappedComponent :type "PrimitiveComponent Object Reference") (OtherActor :type "Actor Object Reference") (OtherComp :type "PrimitiveComponent Object Reference") (OtherBodyIndex :type Integer))
  (cast `/Game/VR_BP/MotionControllerPawn` OtherActor)
  (`SceneComponent.SetVisibility` (`self.Hint`) false false)
  (set `self.IsOverLapped?` false))

(fn `UserConstructionScript`)